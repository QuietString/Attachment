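; BP_AttachmentManager is a test Blueprint that reverses the attachment hierarchy between two referenced actors, Parent and Child, under a Root actor.
; SwapParentAndChild validates all three references, attaches Child to Root, then attaches Parent to Child, keeping relative transforms.
; If the second attach succeeds, it swaps the references and prints the change; otherwise it prints a failure message in red.
; Nothing in the file calls the function.
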(fn `Swap Parent And Child`
  (locals (PrevParent :type "Actor Object Reference") (DebugMessage :type String) (PrevChild :type "Actor Object Reference"))
  (`/Engine/EditorBlueprintResources/StandardMacros.IsValid` (`self.Parent`)
    (:`Is Valid`
      (`/Engine/EditorBlueprintResources/StandardMacros.IsValid` (`self.Child`)
        (:`Is Valid`
          (`/Engine/EditorBlueprintResources/StandardMacros.IsValid` (`self.Root`)
            (:`Is Valid`
              (`SceneComponent.K2_AttachToComponent` (`Actor.RootComponent` (`self.Child`)) (`Actor.RootComponent` (`self.Root`)) "None" "KeepRelative" "KeepRelative" "KeepRelative" true)
              (bind _returnvalue (`SceneComponent.K2_AttachToComponent` (`Actor.RootComponent` (`self.Parent`)) (`Actor.RootComponent` (`self.Child`)) "None" "KeepRelative" "KeepRelative" "KeepRelative" true))
              (if _returnvalue
                (set `local.PrevParent` (`self.Parent`))
                (set `local.PrevChild` (`self.Child`))
                (set `self.Parent` (`self.Child`))
                (set `self.Child` (`local.PrevParent`))
                (`KismetSystemLibrary.PrintString` (`KismetStringLibrary.Concat_StrStr` "Parent changed from " (`KismetSystemLibrary.GetDisplayName` (`local.PrevParent`)) " to " (`KismetSystemLibrary.GetDisplayName` (`self.Parent`)) ", child changed from " (`KismetSystemLibrary.GetDisplayName` (`local.PrevChild`)) " to " (`KismetSystemLibrary.GetDisplayName` (`self.Child`))) true true (struct :`G` 0.66 :`B` 1.0 :`A` 1.0) 10.0)
                (else
                  (`KismetSystemLibrary.PrintString` "Failed to swap parent and child" true true (struct :`R` 1.0 :`A` 1.0) :!label _label))))
            (:`Is Not Valid`
              (goto _label))))
        (:`Is Not Valid`
          (goto _label))))
    (:`Is Not Valid`
      (goto _label))))

(fn `UserConstructionScript`)